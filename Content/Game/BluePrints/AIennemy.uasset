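; Enemy pawn, apparently for a tower defense game, that walks to the first TargetPoint found, then destroys itself, damages the My_Camera player and increments its Kill count.
; LooseHp subtracts health, returns whether it survives, and on death awards money, score and a kill.
; BeginPlay links the health widget, Tick swaps the sphere material by health ratio, and cursor hover shows current health as text.
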(event `self.ReceiveBeginPlay`
  (bind _asennemis_hp (cast `/Game/Game/HUD/Ennemis_hp` (`WidgetComponent.GetUserWidgetObject` (`self.Health`))))
  (set `/Game/Game/HUD/Ennemis_hp.Ennemy` self _asennemis_hp)
  (set `self.MaxVie` (`self.Vie`))
  (`KismetSystemLibrary.Delay` 0.2)
  (bind _outactors (`GameplayStatics.GetAllActorsOfClass` "/Script/Engine.TargetPoint"))
  (`|AIMoveTo` self (0.0 0.0 0.0) (`|GetArrayItem` _outactors)
    (:`OnSuccess`
      (`self.K2_DestroyActor`)
      (bind _asmy_camera (cast `/Game/Game/BluePrints/My_Camera` (`GameplayStatics.GetPlayerCharacter` 0)))
      (`/Game/Game/BluePrints/My_Camera.TakeDamage` _asmy_camera 0.1)
      (set `/Game/Game/BluePrints/My_Camera.Kill` (+ (`/Game/Game/BluePrints/My_Camera.Kill` _asmy_camera) 1) _asmy_camera))))

(event `self.ReceiveTick`
  (params (DeltaSeconds :type "Float (single-precision)"))
  (bind _test (`self.Test`))
  (bind _sphere (`self.Sphere`))
  (set `self.Test` (/ (`self.Vie`) (`self.MaxVie`)))
  (if (>= _test 1.0)
    (`PrimitiveComponent.SetMaterial` _sphere 0 "/Game/Game/BluePrints/Health/Health10.Health10")
    (elif (>= _test 0.9)
      (`PrimitiveComponent.SetMaterial` _sphere 0 "/Game/Game/BluePrints/Health/Health9.Health9")
      (elif (>= _test 0.8)
        (`PrimitiveComponent.SetMaterial` _sphere 0 "/Game/Game/BluePrints/Health/Health8.Health8")
        (elif (>= _test 0.7)
          (`PrimitiveComponent.SetMaterial` _sphere 0 "/Game/Game/BluePrints/Health/Health7.Health7")
          (elif (>= _test 0.6)
            (`PrimitiveComponent.SetMaterial` _sphere 0 "/Game/Game/BluePrints/Health/Health6.Health6")
            (elif (>= _test 0.5)
              (`PrimitiveComponent.SetMaterial` _sphere 0 "/Game/Game/BluePrints/Health/Health5.Health5")
              (elif (>= _test 0.4)
                (`PrimitiveComponent.SetMaterial` _sphere 0 "/Game/Game/BluePrints/Health/Health4.Health4")
                (elif (>= _test 0.3)
                  (`PrimitiveComponent.SetMaterial` _sphere 0 "/Game/Game/BluePrints/Health/Health3.Health3")
                  (elif (>= _test 0.2)
                    (`PrimitiveComponent.SetMaterial` _sphere 0 "/Game/Game/BluePrints/Health/Health2.Health2")
                    (elif (>= _test 0.0)
                      (`PrimitiveComponent.SetMaterial` _sphere 0 "/Game/Game/BluePrints/Health/Health1.Health1"))))))))))))

(event `self.Sphere.OnBeginCursorOver`
  (params (TouchedComponent :type "PrimitiveComponent Object Reference"))
  (`TextRenderComponent.K2_SetText` (`self.TextRender`) (`KismetTextLibrary.Conv_DoubleToText` (`self.Vie`) "HalfToEven")))

(event `self.Sphere.OnEndCursorOver`
  (params (TouchedComponent :type "PrimitiveComponent Object Reference"))
  (`TextRenderComponent.K2_SetText` (`self.TextRender`) (`KismetTextLibrary.Conv_StringToText` "")))

(fn `Loose_Hp`
  (params (Value :type "Float (double-precision)"))
  (returns (`Life?` :type Boolean))
  (bind _output_get (set `self.Vie` (- (`self.Vie`) Value)))
  (if (<= _output_get 0.0)
    (`self.K2_DestroyActor`)
    (bind _asmy_camera (cast `/Game/Game/BluePrints/My_Camera` (`GameplayStatics.GetPlayerCharacter` 0)))
    (`/Game/Game/BluePrints/My_Camera.AddMoney` _asmy_camera (`self.argent`))
    (bind _asmy_camera_2 (cast `/Game/Game/BluePrints/My_Camera` (`GameplayStatics.GetPlayerCharacter` 0)))
    (`/Game/Game/BluePrints/My_Camera.AddScore` _asmy_camera_2 (`self.scoring`))
    (set `/Game/Game/BluePrints/My_Camera.Kill` (+ (`/Game/Game/BluePrints/My_Camera.Kill` _asmy_camera_2) 1) _asmy_camera_2)
    (return false)
    (else
      (return true))))

(fn `UserConstructionScript`)