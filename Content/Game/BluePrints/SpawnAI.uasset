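; SpawnAI is an enemy wave spawner that runs a fixed, scripted sequence of AIennemy spawns when play begins.
; BeginPlay chains Delay nodes between calls to Spawn, producing waves of weak enemies, a lone tougher one, then a final wave of rising health.
; Spawn creates each AIennemy at a hard-coded location and sets its current and max health, money (Argent) and score values from the call's parameters.
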(event `self.ReceiveBeginPlay`
  (`KismetSystemLibrary.Delay` 1.5)
  (`self.Spawn` 10.0 2 1)
  (`KismetSystemLibrary.Delay` 1.0)
  (`self.Spawn` 10.0 2 1)
  (`KismetSystemLibrary.Delay` 1.0)
  (`self.Spawn` 10.0 2 1)
  (`KismetSystemLibrary.Delay` 1.0)
  (`self.Spawn` 10.0 2 1)
  (`KismetSystemLibrary.Delay` 20.0)
  (`self.Spawn` 50.0 5 2)
  (`KismetSystemLibrary.Delay` 20.0)
  (`self.Spawn` 10.0 2 1)
  (`KismetSystemLibrary.Delay` 1.0)
  (`self.Spawn` 10.0 2 1)
  (`KismetSystemLibrary.Delay` 1.5)
  (`self.Spawn` 15.0 2 1)
  (`KismetSystemLibrary.Delay` 1.0)
  (`self.Spawn` 15.0 2 1)
  (`KismetSystemLibrary.Delay` 1.5)
  (`self.Spawn` 20.0 2 1)
  (`KismetSystemLibrary.Delay` 1.0)
  (`self.Spawn` 20.0 2 1))

(fn `Spawn`
  (params (Hp :type "Float (double-precision)") (Argent :type Integer) (Scoring :type Integer))
  (bind _returnvalue (`AIBlueprintHelperLibrary.SpawnAIFromClass` "/Game/Game/BluePrints/AIennemy.AIennemy_C" null (-5800.0 3715.0 170.0)))
  (bind _asaiennemy (cast `/Game/Game/BluePrints/AIennemy` _returnvalue))
  (set `/Game/Game/BluePrints/AIennemy.Vie` Hp _asaiennemy)
  (bind _asaiennemy_2 (cast `/Game/Game/BluePrints/AIennemy` _returnvalue))
  (set `/Game/Game/BluePrints/AIennemy.MaxVie` Hp _asaiennemy_2)
  (bind _asaiennemy_3 (cast `/Game/Game/BluePrints/AIennemy` _returnvalue))
  (set `/Game/Game/BluePrints/AIennemy.argent` Argent _asaiennemy_3)
  (bind _asaiennemy_4 (cast `/Game/Game/BluePrints/AIennemy` _returnvalue))
  (set `/Game/Game/BluePrints/AIennemy.scoring` Scoring _asaiennemy_4))

(fn `UserConstructionScript`)